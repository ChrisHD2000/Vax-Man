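; Pac-Man actor Blueprint that switches which of four directional components (Up, Down, Left, Right) is visible to match keyboard input.
; BeginPlay hides all but Left, leaving it at its default visibility.
; WASD and arrow keys share one handler per direction, each showing that component and hiding the other three.
; It uses direct key events and contains no movement logic.
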(event `self.ReceiveBeginPlay`
  (`SceneComponent.SetVisibility` (`self.Down`) false false)
  (`SceneComponent.SetVisibility` (`self.Right`) false false)
  (`SceneComponent.SetVisibility` (`self.Up`) false false))

(event `Key|W`
  (params (Key :type "Key Structure"))
  (:`Pressed`
    (`SceneComponent.SetVisibility` (`self.Down`) false false :!label _label)
    (`SceneComponent.SetVisibility` (`self.Right`) false false)
    (`SceneComponent.SetVisibility` (`self.Left`) false false)
    (`SceneComponent.SetVisibility` (`self.Up`) true false)))

(event `Key|Up`
  (params (Key :type "Key Structure"))
  (:`Pressed`
    (goto _label)))

(event `Key|S`
  (params (Key :type "Key Structure"))
  (:`Pressed`
    (`SceneComponent.SetVisibility` (`self.Right`) false false :!label _label_2)
    (`SceneComponent.SetVisibility` (`self.Left`) false false)
    (`SceneComponent.SetVisibility` (`self.Up`) false false)
    (`SceneComponent.SetVisibility` (`self.Down`) true false)))

(event `Key|Down`
  (params (Key :type "Key Structure"))
  (:`Pressed`
    (goto _label_2)))

(event `Key|D`
  (params (Key :type "Key Structure"))
  (:`Pressed`
    (`SceneComponent.SetVisibility` (`self.Up`) false false :!label _label_3)
    (`SceneComponent.SetVisibility` (`self.Down`) false false)
    (`SceneComponent.SetVisibility` (`self.Left`) false false)
    (`SceneComponent.SetVisibility` (`self.Right`) true false)))

(event `Key|Right`
  (params (Key :type "Key Structure"))
  (:`Pressed`
    (goto _label_3)))

(event `Key|A`
  (params (Key :type "Key Structure"))
  (:`Pressed`
    (`SceneComponent.SetVisibility` (`self.Up`) false false :!label _label_4)
    (`SceneComponent.SetVisibility` (`self.Down`) false false)
    (`SceneComponent.SetVisibility` (`self.Right`) false false)
    (`SceneComponent.SetVisibility` (`self.Left`) true false)))

(event `Key|Left`
  (params (Key :type "Key Structure"))
  (:`Pressed`
    (goto _label_4)))

(fn `UserConstructionScript`)